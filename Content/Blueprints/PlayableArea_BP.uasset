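; Playable area actor for an Asteroids game that provides the view camera, screen wrapping, and asteroid and UFO spawning.
; It sizes its box to the screen edges at z=0 from camera FOV and height, updates on aspect changes, and shares the extent through Asteroids_GS.
; Actors leaving the box warp across, or are destroyed if tagged doNotWarp.
; GameState events drive spawning near the edges, with UFOs on a self-restarting random timer.
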(event OnComponentEndOverlap(Box)
  (params (OverlappedComponent :type Primitive%20Component%20Object%20Reference) (OtherActor :type Actor%20Object%20Reference) (OtherComp :type Primitive%20Component%20Object%20Reference) (OtherBodyIndex :type Integer))
  ;[1 1 1] When an actor leaves the playable area, warp it to the other side.
  (CallFunction|Warp OtherActor))

(event Custom|Start%20Game
  (CallFunction|SpawnAsteroids)
  (CallFunction|SpawnUFOHelper))

(event Custom|End%20Game
  ;[1 1 1] Clear timers
  (Utilities|Time|ClearTimerbyFunctionName 0 "SpawnUFOHelper")
  (Utilities|Time|ClearTimerbyFunctionName 0 "SpawnAsteroids"))

(event EventBeginPlay
  (Utilities|FlowControl|Sequence
    (:then_0
      ;[1 1 1] Bind GameState events.
      (bind _asasteroids_gs (Utilities|Casting|CastToAsteroids_GS (Game|GetGameState)))
      (EventDispatchers|BindEventtoWaveComplete _asasteroids_gs (EventDispatchers|CreateEvent :!event SpawnAsteroids))
      (EventDispatchers|BindEventtoStartGame _asasteroids_gs (EventDispatchers|CreateEvent :!event Custom|Start%20Game))
      (EventDispatchers|BindEventtoEndGame _asasteroids_gs (EventDispatchers|CreateEvent :!event Custom|End%20Game)))
    (:then_1
      ;[1 1 1] Set the active camera to our camera
      (Game|Player|SetViewTargetwithBlend (Game|GetPlayerController 0) self 0.0 "VTBlend_Linear" 0.0 false)
      (CallFunction|CalculatePlayableArea))
    (:then_2
      (CallFunction|SpawnAsteroids) ; Spawn some asteroids\nto make the game feel alive.
    )))

(event EventTick
  (params (DeltaSeconds :type Float%20%28single-precision%29))
  (bind _returnvalue (Viewport|GetViewportSize))
  (bind (_x _y) (Math|Vector2D|BreakVector2D _returnvalue))
  ;[1 1 1] Each frame, check to see if the resolution changes.
  ; If it does, recalculate the playable area.
  (if (!= (Variables|Default|GetPlayableAreaRatio) (/ _x _y))
    (CallFunction|CalculatePlayableArea)))

(fn ConstructionScript)

(fn CalculatePlayableArea
  (bind _returnvalue (Viewport|GetViewportSize))
  (bind _camera (Variables|Default|GetCamera))
  (bind _returnvalue_2 (Transformation|GetWorldLocation _camera))
  (bind (_x _y) (Math|Vector2D|BreakVector2D _returnvalue))
  (bind _fieldofview (Variables|/Script/Engine.CameraComponent|GetFieldOfView _camera))
  (bind _z (Class|KismetMathLibrary|BreakVector3f _returnvalue_2))
  (bind _returnvalue_3 (/ _fieldofview 2.0))
  (bind _returnvalue_4 (/ _x _y))
  (bind _returnvalue_5 (Math|Trig|Tan(Degrees) _returnvalue_3))
  (bind _returnvalue_6 (* _returnvalue_5 _z))
  (bind _asasteroids_gs (Utilities|Casting|CastToAsteroids_GS (Game|GetGameState))) ; Wrap size is stored in Asteroids_GS
  (bind _output_get (Variables|/Game/Blueprints/Asteroids_GS.Asteroids_GS_C|SetWrap _asasteroids_gs (Math|Vector|MakeVector (/ _returnvalue_6 _returnvalue_4) _returnvalue_6 1e+03)))
  (Components|Box|SetBoxExtent (Variables|Default|GetBox) _output_get true)
  (Variables|Default|SetPlayableAreaRatio _returnvalue_4))

(fn SpawnUFOHelper
  (if (Class|KismetSystemLibrary|TimerExists 0 "SpawnUFOHelper") ; If the timer exists,\nthen spawn a UFO,\notherwise start the timer.
    ;[1 1 1] Store the GameState as an Asteroids_GS
    (bind _asasteroids_gs (Utilities|Casting|CastToAsteroids_GS (Game|GetGameState)))
    (LocalVariables|SetGameState _asasteroids_gs)
    ;[1 1 1] Check if the GameState will allow a new UFO
    (if (Default|CanSpawnUFO (LocalVariables|GetGameState))
      (Utilities|FlowControl|Sequence
        (:then_0
          ;[1 1 1] Generate a spawn location somewhere on the edge of the screen.
          (LocalVariables|SetSpawnLocation (select (Math|Random|RandomBool) (Math|Vector|MakeVector (.X (Class|KismetMathLibrary|BreakVector3f (Math|Vector|SelectVector (* (Variables|/Game/Blueprints/Asteroids_GS.Asteroids_GS_C|GetWrap (LocalVariables|GetGameState)) -1.0) (Variables|/Game/Blueprints/Asteroids_GS.Asteroids_GS_C|GetWrap (LocalVariables|GetGameState)) (Math|Random|RandomBool)))) (.Y (Math|Vector|BreakVector (* (Variables|/Game/Blueprints/Asteroids_GS.Asteroids_GS_C|GetWrap (LocalVariables|GetGameState)) (Math|Random|RandomFloatinRange -1.0 1.0)))) 0.0) (Math|Vector|MakeVector (.X (Math|Vector|BreakVector (* (Variables|/Game/Blueprints/Asteroids_GS.Asteroids_GS_C|GetWrap (LocalVariables|GetGameState)) (Math|Random|RandomFloatinRange -1.0 1.0)))) (.Y (Class|KismetMathLibrary|BreakVector3f (Math|Vector|SelectVector (* (Variables|/Game/Blueprints/Asteroids_GS.Asteroids_GS_C|GetWrap (LocalVariables|GetGameState)) -1.0) (Variables|/Game/Blueprints/Asteroids_GS.Asteroids_GS_C|GetWrap (LocalVariables|GetGameState)) (Math|Random|RandomBool)))) 0.0))))
        (:then_1
          ;[1 1 1] Spawn UFO
          (Game|SpawnActorfromClass "/Game/Blueprints/UFO_Blueprint.UFO_Blueprint_C" (Math|Transform|MakeTransform (LocalVariables|GetSpawnLocation)) "Undefined" 0 (* (Math|Vector|Normalize (LocalVariables|GetSpawnLocation)) -1.0) (Math|Random|RandomBool) 0))
        (:then_2
          (Utilities|Time|SetTimerbyFunctionName 0 "SpawnUFOHelper" (Math|Random|RandomFloatinRange 1.0 6e+01) :!label _label) ; Restart the timer.
        ))
      (else
        (goto _label)))
    (else
      (goto _label))))

(fn SpawnAsteroids
  (bind _returnvalue (Math|Random|RandomFloatinRange 0.0 0.95))
  (bind _returnvalue_2 (Math|Random|RandomBool))
  (bind _asasteroids_gs (Utilities|Casting|CastToAsteroids_GS (Game|GetGameState)))
  (for _index (range 1 (Variables|/Game/Blueprints/Asteroids_GS.Asteroids_GS_C|GetCurrentAsteroids _asasteroids_gs)) ; Spawn "CurrentAsteroids" asteroids.
    (Game|SpawnActorfromClass "/Game/Blueprints/Asteroid_Blueprint.Asteroid_Blueprint_C" (Math|Transform|MakeTransform (* (Variables|/Game/Blueprints/Asteroids_GS.Asteroids_GS_C|GetWrap _asasteroids_gs) 0.95 (Math|Vector|MakeVector (Math|Float|SelectFloat _returnvalue 1.0 _returnvalue_2) (Math|Float|SelectFloat 1.0 _returnvalue _returnvalue_2) 0.0) (Math|Vector|MakeVector (Math|Float|SelectFloat 1.0 -1.0 (Math|Random|RandomBool)) (Math|Float|SelectFloat 1.0 -1.0 (Math|Random|RandomBool)) 0.0))) "Undefined" 0 (LocalVariables|GetInitialHits) (* (Math|Vector|RotateVectorAroundAxis (Class|KismetMathLibrary|VectorForward) (Math|Random|RandomFloatinRange 0.0 3.6e+02) (Math|Vector|VectorUp)) (LocalVariables|GetInitialSpeed)) 0)))

(fn Warp
  (params (ActorToWarp :type Actor%20Object%20Reference))
  (if (Actor|ActorHasTag ActorToWarp "doNotWarp") ; If an actor does not warp,\ndestroy it instead.
    (Actor|DestroyActor ActorToWarp)
    (else
      ;[1 1 1] Warp actor.
      (bind _asasteroids_gs (Utilities|Casting|CastToAsteroids_GS (Game|GetGameState)))
      (Transformation|SetActorLocation ActorToWarp (Utilities|WarpCalculator (Transformation|GetActorLocation ActorToWarp) (Variables|/Game/Blueprints/Asteroids_GS.Asteroids_GS_C|GetWrap _asasteroids_gs)) false true))))