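; Game State for an Asteroids game that runs game start and end, waves, and coordinated pausing, broadcasting each change.
; It tracks asteroids, UFOs and other registered actors in sets, clearing all on a new game.
; Removing an asteroid or UFO checks for wave end, which raises the asteroid count up to a cap and announces completion after a delay.
; It also gates UFO spawning to one at a time while asteroids remain.
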(event Custom|Intermission
  (Default|CallWaveComplete) ; Broadcast that\na wave has been completed.
)

(event Custom|End%20Game
  (Variables|Default|SetGameActive false) ; A game is no longer active.
  (CallFunction|UnpauseGame) ; Unpause just in case.
  (Default|CallEndGame) ; Broadcast that\na game has ended
)

(event Custom|Wave%20Complete
  (Variables|Default|SetCurrentAsteroids (Math|Integer|Min(Integer) (+ (Variables|Default|GetCurrentAsteroids) 2) (Variables|Default|GetMaxAsteroids))) ; Set the new number of\nasteroids this wave.
  (Utilities|Time|SetTimerbyFunctionName 0 "Intermission" 3.0) ; Give the player some time \nbefore starting the next wave.
)

(event Custom|Unpause%20Game
  ;[1 1 1] All pausing is done from here so that everyone can coordinate their pause responses.
  (Game|SetGamePaused false)
  (Default|CallGameUnpaused))

(event Custom|Pause%20Game
  ;[1 1 1] All pausing is done from here so that everyone can coordinate their pause responses.
  (Game|SetGamePaused true)
  (Default|CallGamePaused))

(event Custom|Check%20Wave%20End
  (if (and (<= (Utilities|Set|Length (Variables|Default|GetActiveAsteroids)) 0) (<= (Utilities|Set|Length (Variables|Default|GetActiveUFOs)) 0)) ; If there are no asteroids and no UFOs\nthen a wave has been completed.
    (CallFunction|WaveComplete)))

(event Custom|Start%20Game
  (if (not (Variables|Default|GetGameActive)) ; Don't start a game\nif one is already active.
    (Variables|Default|SetCurrentAsteroids (Variables|Default|GetInitialAsteroids)) ; Set initial asteroids.
    (Variables|Default|SetGameActive true) ; A game is now active.
    (CallFunction|ClearAll) ; Remove all actors\nfrom the playing field.
    (Default|CallStartGame) ; Broadcast that\na game is has started.
  ))

(event Custom|Remove%20Asteroid
  (params (Asteroid :type Actor%20Object%20Reference))
  ;[1 1 1] Tracking of asteroids
  (Utilities|Set|Remove (Variables|Default|GetActiveAsteroids) Asteroid)
  (Utilities|FlowControl|Sequence
    (:then_0
      ;[1 1 1] Whenever a UFO or an Asteroid is untracked (Destroyed), we should check to see if the wave has ended.
      (CallFunction|CheckWaveEnd))
    (:then_1
      (Default|CallNumberOfAsteroidsUpdated (Utilities|Set|Length (Variables|Default|GetActiveAsteroids))) ; Broadcast that the number of\nasteroids has changed
    )))

(event Custom|Add%20Asteroid
  (params (Asteroid :type Actor%20Object%20Reference))
  ;[1 1 1] Tracking of asteroids
  (Utilities|Set|Add (Variables|Default|GetActiveAsteroids) Asteroid)
  (Default|CallNumberOfAsteroidsUpdated (Utilities|Set|Length (Variables|Default|GetActiveAsteroids))) ; Broadcast that the number of\nasteroids has changed
)

(event Custom|Remove%20UFO
  (params (UFO :type Actor%20Object%20Reference))
  ;[1 1 1] Tracking of UFO
  (Utilities|Set|Remove (Variables|Default|GetActiveUFOs) UFO)
  ;[1 1 1] Whenever a UFO or an Asteroid is untracked (Destroyed), we should check to see if the wave has ended.
  (CallFunction|CheckWaveEnd))

(event Custom|Add%20UFO
  (params (UFO :type Actor%20Object%20Reference))
  ;[1 1 1] Tracking of UFO
  (Utilities|Set|Add (Variables|Default|GetActiveUFOs) UFO))

(event EventRegister
  (params (Actor :type Actor%20Object%20Reference))
  ;[1 1 1] Tracking of insignificant actors that should be cleared when a new game starts.
  (Utilities|Set|Add (Variables|Default|GetOtherActors) Actor))

(event EventUnregister
  (params (Actor :type Actor%20Object%20Reference))
  ;[1 1 1] Tracking of insignificant actors that should be cleared when a new game starts.
  (Utilities|Set|Remove (Variables|Default|GetOtherActors) Actor))

(event Custom|Clear%20OtherActors
  ;[1 1 1] Destroy each actor in each of these sets
  (CallFunction|ClearSet (Variables|Default|GetOtherActors)))

(event Custom|Clear%20Asteroids
  ;[1 1 1] Destroy each actor in each of these sets
  (CallFunction|ClearSet (Variables|Default|GetActiveAsteroids)))

(event Custom|Clear%20UFOs
  ;[1 1 1] Destroy each actor in each of these sets
  (CallFunction|ClearSet (Variables|Default|GetActiveUFOs)))

(event Custom|Clear%20All
  (CallFunction|ClearAsteroids)
  (CallFunction|ClearUFOs)
  (CallFunction|ClearOtherActors))

(fn ConstructionScript
  (Variables|Default|SetCurrentAsteroids (Variables|Default|GetInitialAsteroids)))

(fn CanSpawnUFO
  ;[1 1 1] A UFO should only be spawned if there isn't currently a UFO and there are still asteroids present.
  (return (and (Utilities|Set|IsEmpty (Variables|Default|GetActiveUFOs)) (Utilities|Set|IsNotEmpty (Variables|Default|GetActiveAsteroids)))))

(fn ClearSet
  (params (Set :type Set%20of%20Actor%20Object%20References))
  (bind _result (Utilities|Set|ToArray Set))
  (for _array_element _result
    (EventDispatchers|UnbindallEventsfromOnDestroyed _array_element) ; Override special destroy handling
    (Actor|DestroyActor _array_element))
  (Utilities|Set|Clear Set))