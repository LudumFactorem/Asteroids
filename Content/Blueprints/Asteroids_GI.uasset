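; Game instance for an Asteroids game that owns the Master, Music and SFX volume settings, loading and applying them on Init.
; A map of sound classes to volumes feeds sound class overrides on the Master_Mix sound mix.
; Values save to and load from an OptionsSave slot.
; When loading fails, defaults come from a data table, and resetting broadcasts VolumesChanged after applying them.
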(event EventInit
  (CallFunction|LoadVolume) ; Load volume settings
  (CallFunction|UpdateVolume) ; Apply volume settings
)

(fn SetVolume
  (params (Class :type Sound%20Class%20Object%20Reference) (Volume :type Float%20%28double-precision%29))
  (Utilities|Map|Add (Variables|Default|GetVolumeSettings) Class Volume))

(fn SaveVolume
  (bind _volumesettings (Variables|Default|GetVolumeSettings))
  ;[1 1 1] Prepare the data we want to save
  (bind _returnvalue (Game|ConstructObjectfromClass "/Game/Blueprints/OptionsSave.OptionsSave_C" (Utilities|Struct|MakeVolume (.Value (Utilities|Map|Find _volumesettings "/Engine/EngineSounds/Master.Master")) (.Value (Utilities|Map|Find _volumesettings "/Engine/EngineSounds/Music.Music")) (.Value (Utilities|Map|Find _volumesettings "/Engine/EngineSounds/SFX.SFX")))))
  ;[1 1 1] Save the data
  (bind _returnvalue_2 (SaveGame|SaveGametoSlot _returnvalue (Variables|Default|GetSettingsSlot)))
  (if _returnvalue_2
    (Development|PrintString "Settings saved.")
    (else
      (Development|PrintString "Failed to save settings." true true "(R=1.000000,G=0.591212,B=0.000000,A=1.000000)" 4.0))))

(fn UpdateVolume
  ;[1 1 1] Iterate through VolumeSettings, applying each of them.
  (bind _keys (Utilities|Map|Keys (Variables|Default|GetVolumeSettings)))
  (for _array_element _keys
    (Audio|SetSoundMixClassOverride "/Game/Audio/Master_Mix.Master_Mix" _array_element (.Value (Utilities|Map|Find (Variables|Default|GetVolumeSettings) _array_element)) 1.0 0.0 true)))

(fn LoadVolume
  ;[1 1 1] Load the settings file
  (bind _returnvalue (SaveGame|LoadGamefromSlot (Variables|Default|GetSettingsSlot)))
  (bind _asoptions_save (Utilities|Casting|CastToOptionsSave _returnvalue)
    (:then
      ;[1 1 1] Get the settings from the save file and store them accordingly
      (Utilities|FlowControl|Sequence
        (:then_0
          (CallFunction|SetVolume "/Engine/EngineSounds/Master.Master" (.Master (Utilities|Struct|BreakVolume (Variables|/Game/Blueprints/OptionsSave.OptionsSave_C|GetVolumeSettings _asoptions_save)))))
        (:then_1
          (CallFunction|SetVolume "/Engine/EngineSounds/Music.Music" (.Music (Utilities|Struct|BreakVolume (Variables|/Game/Blueprints/OptionsSave.OptionsSave_C|GetVolumeSettings _asoptions_save)))))
        (:then_2
          (CallFunction|SetVolume "/Engine/EngineSounds/SFX.SFX" (.Sounds (Utilities|Struct|BreakVolume (Variables|/Game/Blueprints/OptionsSave.OptionsSave_C|GetVolumeSettings _asoptions_save)))))))
    (:CastFailed
      (CallFunction|ResetVolumes) ; No settings file found.\nSetting defaults
    )))

(fn GetVolume
  (params (Class :type Sound%20Class%20Object%20Reference))
  (return (.Value (Utilities|Map|Find (Variables|Default|GetVolumeSettings) Class))))

(fn ResetVolumes
  (bind _outrownames (DataTable|GetDataTableRowNames (Variables|Default|GetVolumeDefaultsTable))) ; Default settings\nare stored in a data table
  ;[1 1 1] Set each of the volume settings to the default found in the data table
  (for _array_element _outrownames
    (bind _returnvalue (Utilities|GetDataTableRow (Variables|Default|GetVolumeDefaultsTable) _array_element)
      (:then
        (CallFunction|SetVolume (.SoundClass (Utilities|Struct|BreakVolumeDefault _returnvalue)) (.Volume (Utilities|Struct|BreakVolumeDefault _returnvalue))))))
  (CallFunction|UpdateVolume)
  (Default|CallVolumesChanged) ; Broadcast that the volume settings\nwere changed programatically
)