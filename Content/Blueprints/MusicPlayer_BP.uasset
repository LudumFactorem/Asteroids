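; Music player actor that speeds up the game's music as the number of asteroids grows.
; On BeginPlay it binds to the asteroid count update event on Asteroids_GS and activates its audio component.
; Each update sets the audio's Speed parameter to the asteroid count divided by a fixed constant.
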(event Custom|Update%20Music%20Speed
  (params (Asteroids :type Integer))
  ;[1 1 1] Play the music more quickly when there are more asteroids.
  (Audio|Parameter|SetFloatParameter (Variables|Default|GetAudio) "Speed" (/ (Math|Conversions|ToFloat(Integer) Asteroids) 32.0) :!class /Script/AudioExtensions.AudioParameterControllerInterface))

(event EventBeginPlay
  (Utilities|FlowControl|Sequence
    (:then_0
      (bind _asasteroids_gs (Utilities|Casting|CastToAsteroids_GS (Game|GetGameState)))
      (EventDispatchers|BindEventtoNumberOfAsteroidsUpdated _asasteroids_gs (EventDispatchers|CreateEvent :!event Custom|Update%20Music%20Speed)))
    (:then_1
      (Components|Activation|Activate (Variables|Default|GetAudio) false))))

(fn ConstructionScript)