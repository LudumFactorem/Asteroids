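; Player spaceship pawn for an Asteroids-style game, driven through controller interface events and registered with the GameState.
; A physics sphere handles turning and thrust, while a thruster map derived from both inputs toggles four thrusters and their audio.
; PlayerState limits live projectiles, which are tagged to destroy aliens.
; Teleport respawns through a spawner actor; "shipDestroyer" hits or self-destruct trigger a one-time death with effects and controller notification.
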(event OnComponentHit(Sphere)
  (params (HitComponent :type Primitive%20Component%20Object%20Reference) (OtherActor :type Actor%20Object%20Reference) (OtherComp :type Primitive%20Component%20Object%20Reference) (NormalImpulse :type Vector :default "0, 0, 0") (Hit :type Hit%20Result%20Structure%20%28by%20ref%29))
  ;[1 1 1] Handle dangerous collisions.
  (if (Utilities|Array|ContainsItem (Variables|/Script/Engine.Actor|GetTags OtherActor) "shipDestroyer")
    (CallFunction|Die)))

(event Custom|Die
  (CallFunction|Deactivate)
  (Utilities|FlowControl|DelayUntilNextTick)
  (Actor|DestroyActor))

(event EventBeginPlay
  (Class|ActorRegistrar|Register(Message) (Game|GetGameState) self))

(event EventDestroyed
  (Class|ActorRegistrar|Unregister(Message) (Game|GetGameState) self))

(event EventTeleport
  (bind _returnvalue (Math|Float|MakeLiteralFloat 0.8))
  (bind _returnvalue_2 (Transformation|GetActorTransform))
  (bind (_location _rotation _scale) (Math|Transform|BreakTransform _returnvalue_2))
  (bind _returnvalue_3 (- 0.0 _returnvalue))
  ;[1 1 1] Teleport the ship to a random location in the playable area.
  ; This is done by spawning a new ship spawner and destroying the current ship.
  (if (Variables|Default|GetAlive)
    (bind _asasteroids_gs (Utilities|Casting|CastToAsteroids_GS (Game|GetGameState)))
    (Game|SpawnActorfromClass "/Game/Blueprints/ShipSpawner.ShipSpawner_C" (Math|Transform|MakeTransform (* (Variables|/Game/Blueprints/Asteroids_GS.Asteroids_GS_C|GetWrap _asasteroids_gs) (Math|Vector|MakeVector (Math|Random|RandomFloatinRange _returnvalue_3 _returnvalue) (Math|Random|RandomFloatinRange _returnvalue_3 _returnvalue) 0.0)) _rotation _scale) "AlwaysSpawn" 0 (Variables|Default|GetTeleportRadius) (Pawn|GetController) 0)
    (Actor|DestroyActor)))

(event EventSelfdestruct
  (CallFunction|Die))

(event EventShoot
  (CallFunction|ShootHelper))

(event EventTurn
  (params (Strength :type Float%20%28double-precision%29))
  (CallFunction|TurnHelper Strength))

(event EventThrust
  (params (Strength :type Float%20%28double-precision%29))
  (CallFunction|ThrustHelper Strength))

(fn ConstructionScript)

(fn TurnHelper
  (params (Strength :type Float%20%28double-precision%29))
  (if (Variables|Default|GetAlive)
    (Utilities|FlowControl|Sequence
      (:then_0
        ;[1 1 1] Turn the ship.
        (Class|PrimitiveComponent|SetPhysicsAngularVelocityinDegrees (Variables|Default|GetSphere) (Math|Vector|MakeVector 0.0 0.0 (* Strength (Variables|Default|GetTurnRate))) false "None"))
      (:then_1
        ;[1 1 1] Store the direction we are turning.
        (Variables|Default|SetDirection (select (== Strength 0.0) "NewEnumerator0" (select (< Strength 0.0) "NewEnumerator1" "NewEnumerator2"))))
      (:then_2
        (CallFunction|UpdateThrusters) ; Update the thrusters.
      ))))

(fn UpdateThrusters
  (Utilities|FlowControl|Sequence
    (:then_0
      ;[1 1 1] Create a map of which thrusters are on and which are off.
      (for _array_element (Utilities|Array|MakeArray (Variables|Default|GetRight_Thruster) (Variables|Default|GetLeft_Thruster) (Variables|Default|GetLeft_Antithruster) (Variables|Default|GetRight_Antithruster))
        (Utilities|Map|Add (LocalVariables|GetThrusterMap) _array_element false)))
    (:then_1
      ;[1 1 1] Parse "Direction" and "Thrusting" to determine which thrusters are on.
      (switch Utilities|FlowControl|Switch|SwitchonTurnMode (Variables|Default|GetDirection)
        (:NewEnumerator0
          (if (Variables|Default|GetThrusting)
            (for _array_element_2 (Utilities|Array|MakeArray (Variables|Default|GetRight_Thruster) (Variables|Default|GetLeft_Thruster)) ; We are not turning,\nbut we are thrusting,\nso turn on the \nleft and right\nthrusters.
              (Utilities|Map|Add (LocalVariables|GetThrusterMap) _array_element_2 true))))
        (:NewEnumerator1
          (Utilities|Map|Add (LocalVariables|GetThrusterMap) (Variables|Default|GetRight_Thruster) true) ; We are turning left\nso turn on the right thruster.
          (if (not (Variables|Default|GetThrusting)) ; When not thrusting,\nturn on the opposite anitthruster\nso that we do not move forward.
            (Utilities|Map|Add (LocalVariables|GetThrusterMap) (Variables|Default|GetLeft_Antithruster) true)))
        (:NewEnumerator2
          (Utilities|Map|Add (LocalVariables|GetThrusterMap) (Variables|Default|GetLeft_Thruster) true) ; We are turning right so\nturn on the left thruster.
          (if (not (Variables|Default|GetThrusting)) ; When not thrusting,\nturn on the opposite antithruster\nso that we do not move forward.
            (Utilities|Map|Add (LocalVariables|GetThrusterMap) (Variables|Default|GetRight_Antithruster) true)))))
    (:then_2
      ;[1 1 1] Apply the new thruster states.
      (bind _keys (Utilities|Map|Keys (LocalVariables|GetThrusterMap)))
      (for _array_element_3 _keys
        (if (.Value (Utilities|Map|Find (LocalVariables|GetThrusterMap) _array_element_3))
          (Components|Activation|Activate _array_element_3 false)
          (else
            (Components|Activation|Deactivate _array_element_3)))))
    (:then_3
      ;[1 1 1] Play a sound so long as even 1 thruster is active.
      (LocalVariables|SetThrusterActive false)
      (bind _values (Utilities|Map|Values (LocalVariables|GetThrusterMap)))
      (bind _array_element_4 (Utilities|Array|ForEachLoopwithBreak _values :!label _label)
        (:LoopBody
          (bind _output_get (LocalVariables|SetThrusterActive (or _array_element_4 (LocalVariables|GetThrusterActive))))
          (if _output_get
            (goto _label Break)))
        (:Completed
          (Class|AudioParameterControllerInterface|SetTriggerParameter (Variables|Default|GetThrusterAudio) (select (LocalVariables|GetThrusterActive) "Engage" "Disengage")))))))

(fn ThrustHelper
  (params (Strength :type Float%20%28double-precision%29))
  (if (Variables|Default|GetAlive)
    (Physics|AddForce (Variables|Default|GetSphere) (* (Transformation|GetActorForwardVector) Strength 1e+03) "None" true)
    (Variables|Default|SetThrusting (> Strength 0.0))
    (CallFunction|UpdateThrusters)))

(fn ShootHelper
  (if (Variables|Default|GetAlive)
    (Utilities|FlowControl|Sequence
      (:then_0
        ;[1 1 1] Fetch Playerstate
        (bind _asplayer_controller (Utilities|Casting|CastToPlayerController (Pawn|GetController)))
        (bind _asasteroids_ps (Utilities|Casting|CastToAsteroids_PS (Variables|/Script/Engine.Controller|GetPlayerState _asplayer_controller)))
        (LocalVariables|SetAsteroidsPS _asasteroids_ps))
      (:then_1
        (Utilities|FlowControl|Sequence
          (:then_0
            ;[1 1 1] Spawn a new projectile (If allowed).
            (if (Default|CanShoot (LocalVariables|GetAsteroidsPS))
              (bind _returnvalue (Game|SpawnActorfromClass "/Game/Blueprints/Projectile.Projectile_C" (Math|Transform|MakeTransform (.Location (Math|Transform|BreakTransform (Transformation|GetWorldTransform (Variables|Default|GetGun))))) "AlwaysSpawn" 0 (Pawn|GetController) self))
              (LocalVariables|SetProjectile _returnvalue)))
          (:then_1
            (Utilities|IsValid (LocalVariables|GetProjectile) ; If a new projectile was spawned\nInitialize it.
              (:Is%20Valid
                ;[1 1 1] Initialize projectile
                (Utilities|FlowControl|Sequence
                  (:then_0
                    (Default|IncrementProjectiles (LocalVariables|GetAsteroidsPS)))
                  (:then_1
                    (Game|BindEventtoOnDestroyed (LocalVariables|GetProjectile) (EventDispatchers|CreateEvent (LocalVariables|GetAsteroidsPS) :!event DecrementProjectiles)) ; Bind the projectile's destruction to the \nplayerstate's decrement projectiles function.
                  )
                  (:then_2
                    (Utilities|Array|Add (Variables|/Script/Engine.Actor|GetTags (LocalVariables|GetProjectile)) "alienDestroyer") ; Enable the projectile to destroy UFO
                  )
                  (:then_3
                    (Physics|SetPhysicsLinearVelocity (Variables|/Game/Blueprints/Projectile.Projectile_C|GetBox (LocalVariables|GetProjectile)) (Default|GetProjectileVelocity (Variables|Default|GetGun)) false "None") ; Send it!
                  )
                  (:then_4
                    (Audio|SpawnSoundatLocation (Variables|Default|GetPewSound) "0, 0, 0" "0, 0, 0" 1.0 1.0 0.0 0 0) ; Play shoot sound.
                  ))))))))))

(fn Deactivate
  (if (Variables|Default|GetAlive) ; Do once and\nturn other features off also.
    (Variables|Default|SetAlive false)
    (Utilities|FlowControl|Sequence
      (:then_0
        ;[1 1 1] Play death particle effect
        (bind _returnvalue (Niagara|SpawnSystematLocation "/Game/Particles/Explode_System.Explode_System" (.Location (Math|Transform|BreakTransform (Transformation|GetActorTransform))) "0, 0, 0" "1.000000,1.000000,1.000000" true false))
        (bind _returnvalue_2 (Physics|GetPhysicsLinearVelocity (Variables|Default|GetSphere) "None"))
        (Effects|Components|ParticleSystem|SetVectorParameter _returnvalue "Velocity" _returnvalue_2)
        (Components|Activation|Activate _returnvalue false))
      (:then_1
        ;[1 1 1] Play death sound effect
        (bind _returnvalue_3 (Audio|SpawnSoundatLocation (Variables|Default|GetDestroySound) "0, 0, 0" "0, 0, 0" 1.0 1.0 0.0 0 0))
        (Audio|Parameter|SetFloatParameter _returnvalue_3 "Pitch" 2.0 :!class /Script/AudioExtensions.AudioParameterControllerInterface)
        (Audio|Parameter|SetFloatParameter _returnvalue_3 "Volume" 1.0 :!class /Script/AudioExtensions.AudioParameterControllerInterface))
      (:then_2
        ;[1 1 1] Deactivate all interactions with the world
        (Physics|SetSimulatePhysics (Variables|Default|GetSphere) false)
        (Collision|SetCollisionEnabled (Variables|Default|GetSphere) "NoCollision")
        (Rendering|SetActorHiddenInGame true)
        (bind _asspaceship_pc (Utilities|Casting|CastToSpaceship_PC (Pawn|GetController)))
        (Default|ShipDestroyed _asspaceship_pc)))))