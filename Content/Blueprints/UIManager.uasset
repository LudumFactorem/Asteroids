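; UI manager that creates the game's widgets at BeginPlay and controls which menu is shown on screen.
; It builds each class in WidgetSetupMap once, caches it by name in WidgetMap, then adds the "ui" widget to the viewport outside the stack.
; Push, Pop and Clear functions drive a menu stack, displaying only the top widget and restoring the previous one on pop.
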(event EventBeginPlay
  (Utilities|FlowControl|Sequence
    (:then_0
      ;[1 1 1] Create menu widgets and store them against a name they can be referenced by.
      (bind _keys (Utilities|Map|Keys (Variables|Default|GetWidgetSetupMap)))
      (for _array_element _keys
        (bind _returnvalue (UserInterface|CreateWidget _array_element (Variables|Default|GetPlayerController)))
        (Utilities|Map|Add (Variables|Default|GetWidgetMap) (.Value (Utilities|Map|Find (Variables|Default|GetWidgetSetupMap) _array_element)) _returnvalue)))
    (:then_1
      ;[1 1 1] Add the ui to the screen.
      (UserInterface|Viewport|AddtoViewport (.Value (Utilities|Map|Find (Variables|Default|GetWidgetMap) "ui")) 0))))

(fn PushMenuWidget
  (params (WidgetName :type Name))
  (bind _menustack (Variables|Default|GetMenuStack))
  (bind _widgetmap (Variables|Default|GetWidgetMap))
  (bind (_value _returnvalue) (Utilities|Map|Find _widgetmap WidgetName))
  (if _returnvalue ; Find the widget.\nIf it doesn't exist,\ndo nothing.
    (LocalVariables|SetWidget _value)
    (Utilities|FlowControl|Sequence
      (:then_0
        ;[1 1 1] Remove the previous widget from its parent.
        (if (Utilities|Array|IsNotEmpty (Variables|Default|GetMenuStack))
          (Widget|RemovefromParent (Utilities|Array|Get(acopy) _menustack (- (Utilities|Array|Length _menustack) 1)))))
      (:then_1
        ;[1 1 1] Add the widget to the stack and display it to the screen.
        (Utilities|Array|Add (Variables|Default|GetMenuStack) (LocalVariables|GetWidget))
        (UserInterface|Viewport|AddtoViewport (LocalVariables|GetWidget) 0)))))

(fn PopMenuWidget
  (if (Utilities|Array|IsNotEmpty (Variables|Default|GetMenuStack)) ; If the menu stack is empty,\nDo nothing
    (LocalVariables|SetEnd (- (Utilities|Array|Length (Variables|Default|GetMenuStack)) 1)) ; Store the top of the stack index
    (Widget|RemovefromParent (Utilities|Array|Get(acopy) (Variables|Default|GetMenuStack) (LocalVariables|GetEnd))) ; Remove the top widget\nfrom its parent
    (Utilities|Array|RemoveIndex (Variables|Default|GetMenuStack) (LocalVariables|GetEnd)) ; Remove the top widget\nfrom the stack
    (if (Utilities|Array|IsNotEmpty (Variables|Default|GetMenuStack)) ; If there is a widget left on the stack\nthen display that.
      (UserInterface|Viewport|AddtoViewport (Utilities|Array|Get(acopy) (Variables|Default|GetMenuStack) (- (LocalVariables|GetEnd) 1)) 0))))

(fn ClearMenu
  (bind _menustack (Variables|Default|GetMenuStack))
  (Utilities|FlowControl|Sequence
    (:then_0
      ;[1 1 1] If there is currently a displayed widget, remove it from its parent (likely the viewport)
      (if (Utilities|Array|IsNotEmpty (Variables|Default|GetMenuStack))
        (Widget|RemovefromParent (Utilities|Array|Get(acopy) _menustack (- (Utilities|Array|Length _menustack) 1)))))
    (:then_1
      (Utilities|Array|Clear (Variables|Default|GetMenuStack)))))