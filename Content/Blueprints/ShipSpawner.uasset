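; ShipSpawner is a placeholder actor that spawns a Spaceship_BP for its Controller once the area is clear, then destroys itself.
; It checks for overlapping physics bodies every frame until the sphere is empty or the radius is too small to matter.
; After a short delay the radius shrinks each tick, with the Sphere component scaled to match.
; It registers with the GameState as a message while alive.
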(event Custom|TrySpawnShip
  (bind _returnvalue (Collision|SphereOverlapActors (Transformation|GetActorLocation) (Variables|Default|GetSpawnCheckRadius) (Utilities|Array|MakeArray "ObjectTypeQuery4") 0)) ; Check if anything is near\nwhere we want to spawn the ship.
  (if (or (< (Variables|Default|GetSpawnCheckRadius) 5e+01) (not _returnvalue))
    ;[1 1 1] Spawn a new ship for the player, and delete myself
    (bind _returnvalue_2 (Game|SpawnActorfromClass "/Game/Blueprints/Spaceship_BP.Spaceship_BP_C" (Transformation|GetActorTransform) "AlwaysSpawn" 0 (- (Variables|Default|GetSpawnCheckRadius) 75.0) 0))
    (Pawn|Possess (Variables|Default|GetController) _returnvalue_2)
    (Actor|DestroyActor)
    (else
      ;[1 1 1] Couldn't spawn ship, try again next frame.
      (Utilities|FlowControl|DelayUntilNextTick)
      (CallFunction|TrySpawnShip))))

(event Custom|Shrink
  ;[1 1 1] Reduce the spawn check radius every tick
  (Variables|Default|SetSpawnCheckRadius (- (Variables|Default|GetSpawnCheckRadius) (* (Utilities|Time|GetWorldDeltaSeconds) (Variables|Default|GetRate))))
  (CallFunction|UpdateScale)
  (Utilities|FlowControl|DelayUntilNextTick)
  (CallFunction|Shrink))

(event EventDestroyed
  (Class|ActorRegistrar|Unregister(Message) (Game|GetGameState) self))

(event EventBeginPlay
  (Class|ActorRegistrar|Register(Message) (Game|GetGameState) self)
  (CallFunction|TrySpawnShip)
  (Utilities|Time|SetTimerbyFunctionName 0 "Shrink" 2.0))

(fn ConstructionScript
  ;[1 1 1] Negative radius produces unwanted results.
  (Variables|Default|SetSpawnCheckRadius (Math|Float|Max(Float) (Variables|Default|GetInitialSpawnCheckRadius) 0.0))
  (CallFunction|UpdateScale))

(fn UpdateScale
  (Transformation|SetRelativeScale3D (Variables|Default|GetSphere) (* "1.000000,1.000000,1.000000" (/ (Variables|Default|GetSpawnCheckRadius) 5e+01))))